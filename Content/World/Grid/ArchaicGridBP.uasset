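; ArchaicGridBP generates the terrain grid map for a turn-based game on BeginPlay.
; A grid macro spawns a cell actor at each point, placing a city at the middle index as the first player fraction's capital.
; Other cells get a terrain class from CellDistribution, which rerolls randomly until it hits a type with remaining quota.
; The finished cell array and dimensions are handed to the TurnBasedController.
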(event EventBeginPlay
  (Variables|Default|SetPlayerFractionRef (Utilities|Array|Get(acopy) (Variables|Default|GetPlayerFractionsArr)))
  (bind (_current_point _total_points _0_1_phase _poly_center) (Utilities|2DGridExecutionMacro 1e+02 (Transformation|GetActorLocation) (Variables|Default|GetDimensionX) (Variables|Default|GetDimensionY))
    (:Per%20Poly%20Execution
      (if (== (/ _total_points 2) _current_point)
        (bind _returnvalue (Game|SpawnActorfromClass "/Game/World/Grid/CityCellBP.CityCellBP_C" (Math|Transform|MakeTransform _poly_center "0, 0, 0" "1,1,1") "Undefined" 0 0 0))
        (Utilities|Array|Add (Variables|Default|GetGridCellArr) _returnvalue)
        (Default|SettingCapital (Variables|Default|GetPlayerFractionRef) _returnvalue)
        (else
          (bind _output (CallFunction|CellDistribution))
          (bind _returnvalue_2 (Game|SpawnActorfromClass (Utilities|Array|Get(acopy) (Variables|Default|GetGridCellClassArr) _output) (Math|Transform|MakeTransform _poly_center "0, 0, 0" "1,1,1") "Undefined" 0 0))
          (Variables|/Game/World/Grid/GridCellBP.GridCellBP_C|SetArchaicGridRef _returnvalue_2 self)
          (Utilities|Array|Add (Variables|Default|GetGridCellArr) _returnvalue_2))))
    (:Output
      (bind _asturn_based_controller (Utilities|Casting|CastToTurnBasedController (Game|GetPlayerController 0)))
      (Variables|/Game/CoreBP/TurnBasedController.TurnBasedController_C|SetGridMapArr _asturn_based_controller (Variables|Default|GetGridCellArr))
      (Variables|/Game/CoreBP/TurnBasedController.TurnBasedController_C|SetDimensionX _asturn_based_controller (Variables|Default|GetDimensionX))
      (Variables|/Game/CoreBP/TurnBasedController.TurnBasedController_C|SetDimensionY _asturn_based_controller (Variables|Default|GetDimensionY)))))

(event Collision|EventActorBeginOverlap
  (params (OtherActor :type Actor%20Object%20Reference)))

(event EventTick
  (params (DeltaSeconds :type Float%20%28single-precision%29)))

(fn ConstructionScript)

(fn CellDistribution
  (while (LocalVariables|GetNeedReroll)
    (bind _output_get (LocalVariables|SetLocalResult (Math|Random|RandomIntegerinRange 0 6)))
    (switch int _output_get
      (:0
        (if (!= (Variables|Counters|GetCountDesert) 0)
          (Variables|Counters|SetCountDesert (- (Variables|Counters|GetCountDesert) 1))
          (LocalVariables|SetNeedReroll false)
          (else
            (LocalVariables|SetNeedReroll true :!label _label))))
      (:1
        (if (!= (Variables|Counters|GetCountPraire) 0)
          (Variables|Counters|SetCountPraire (- (Variables|Counters|GetCountPraire) 1))
          (LocalVariables|SetNeedReroll false)
          (else
            (goto _label))))
      (:2
        (if (!= (Variables|Counters|GetCountMeadow) 0)
          (Variables|Counters|SetCountMeadow (- (Variables|Counters|GetCountMeadow) 1))
          (LocalVariables|SetNeedReroll false)
          (else
            (goto _label))))
      (:3
        (if (!= (Variables|Counters|GetCountForests) 0)
          (Variables|Counters|SetCountForests (- (Variables|Counters|GetCountForests) 1))
          (LocalVariables|SetNeedReroll false)
          (else
            (goto _label))))
      (:4
        (if (!= (Variables|Counters|GetCountHills) 0)
          (Variables|Counters|SetCountHills (- (Variables|Counters|GetCountHills) 1))
          (LocalVariables|SetNeedReroll false)
          (else
            (goto _label))))
      (:5
        (if (!= (Variables|Counters|GetCountMountains) 0)
          (Variables|Counters|SetCountMountains (- (Variables|Counters|GetCountMountains) 1))
          (LocalVariables|SetNeedReroll false)
          (else
            (goto _label))))
      (:6
        (if (!= (Variables|Counters|GetCountLakes) 0)
          (Variables|Counters|SetCountLakes (- (Variables|Counters|GetCountLakes) 1))
          (LocalVariables|SetNeedReroll false)
          (else
            (goto _label))))))
  (return (LocalVariables|GetLocalResult)))