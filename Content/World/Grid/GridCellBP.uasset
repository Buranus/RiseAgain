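; Clickable grid cell for a turn-based strategy map that holds resources, ownership and a building.
; On BeginPlay it derives plant food, fowl, leather and fur yields from its cell type.
; Cursor events toggle hover and ownership decals, and clicking opens the cell menu through the controller's main widget.
; Occupying registers it with the player's fraction and flags overlapped unowned cells as borders; construction spawns a city-linked building that receives the cell's resources when done.
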(event EventBeginPlay
  (bind _celltypeenum (Variables|Default|GetCellTypeEnum))
  (bind _cellfoodefficience (CallFunction|SetPlantFoodEfficience _celltypeenum))
  (bind (_cellfowl _cellleather _cellfur) (CallFunction|SetFowlEfficience _celltypeenum))
  (CallFunction|SetResourceData _cellfoodefficience _cellfowl _cellleather _cellfur "None"))

(event MouseInput|EventActorBeginCursorOver
  ;[1 1 1] Hovering and Clicking Cell handling
  (Rendering|SetVisibility (Variables|Default|GetHoveredDecal) true true))

(event MouseInput|EventActorEndCursorOver
  ;[1 1 1] Hovering and Clicking Cell handling
  (Rendering|SetVisibility (Variables|Default|GetHoveredDecal) false true)
  (if (Variables|CellStateBoolean|GetIsOccupied)
    (Utilities|Casting|CastToCityCellBP self
      (:CastFailed
        (Rendering|SetVisibility (Variables|Default|GetPropertyDecal) true false)))))

(event MouseInput|EventActorOnClicked
  (params (ButtonPressed :type Key%20Structure))
  ;[1 1 1] Hovering and Clicking Cell handling
  (CallFunction|CellRequested))

(fn ConstructionScript)

(fn SetPlantFoodEfficience
  (params (CellType :type CellTypeEnum%20Enum :default "NewEnumerator10"))
  (if (Variables|Default|GetHaveResources)
    (LocalVariables|SetLocalMaxFood 1.2e+02)
    (elif (Math|Boolean|ORBoolean (Utilities|Enum|Equal(Enum) CellType "NewEnumerator10") (Utilities|Enum|Equal(Enum) CellType "NewEnumerator9") (Utilities|Enum|Equal(Enum) CellType "NewEnumerator0") (Utilities|Enum|Equal(Enum) CellType "NewEnumerator11"))
      (LocalVariables|SetLocalMaxFood 0.0)
      (elif (Math|Boolean|ORBoolean (Utilities|Enum|Equal(Enum) CellType "NewEnumerator3") (Utilities|Enum|Equal(Enum) CellType "NewEnumerator8") (Utilities|Enum|Equal(Enum) CellType "NewEnumerator7") (Utilities|Enum|Equal(Enum) CellType "NewEnumerator12"))
        (LocalVariables|SetLocalMaxFood 3e+01)
        (elif (Math|Boolean|ORBoolean (Utilities|Enum|Equal(Enum) CellType "NewEnumerator4") (Utilities|Enum|Equal(Enum) CellType "NewEnumerator5") (Utilities|Enum|Equal(Enum) CellType "NewEnumerator6") (Utilities|Enum|Equal(Enum) CellType "NewEnumerator1"))
          (LocalVariables|SetLocalMaxFood 6e+01)
          (else
            (LocalVariables|SetLocalMaxFood 4e+01))))))
  (return (LocalVariables|GetLocalMaxFood)))

(fn CellRequested
  (bind _asturn_based_controller (Utilities|Casting|CastToTurnBasedController (Game|GetPlayerController 0)))
  (Default|SpawnCellMenu (Variables|/Game/CoreBP/TurnBasedController.TurnBasedController_C|GetMainWidgetRef _asturn_based_controller) self (Variables|/Game/CoreBP/TurnBasedController.TurnBasedController_C|GetPlayerFractionRef _asturn_based_controller))
  (return))

(fn OccupyCell
  (bind _asturn_based_controller (Utilities|Casting|CastToTurnBasedController (Game|GetPlayerController 0)))
  (Utilities|Array|Add (Variables|/Game/Assets/Fractions/FractionBaseBP.FractionBaseBP_C|GetOwnedCellsArr (Variables|/Game/CoreBP/TurnBasedController.TurnBasedController_C|GetPlayerFractionRef _asturn_based_controller)) self)
  (bind _output_get (Variables|Default|SetOccupantFraction (Variables|/Game/CoreBP/TurnBasedController.TurnBasedController_C|GetPlayerFractionRef _asturn_based_controller)))
  (Variables|Default|SetCellBuildingRef (Variables|/Game/Assets/Fractions/FractionBaseBP.FractionBaseBP_C|GetCellBuildingRef _output_get))
  (Variables|CellStateBoolean|SetIsOccupied true)
  (Rendering|SetVisibility (Variables|Default|GetPropertyDecal) true false)
  (CallFunction|CheckingBorderCell)
  (return))

(fn ConstructionDone
  (Default|BuildingPlacing (Variables|Default|GetConstructionRef))
  (Variables|CellStateBoolean|SetIsBuilded true)
  (Variables|/Game/Assets/CellBuildings/CellBuildingBP.CellBuildingBP_C|SetResourcePool (Variables|Default|GetCellBuildingRef) (Variables|Default|GetResourceList))
  (return))

(fn CheckingBorderCell
  (if (Variables|CellStateBoolean|GetIsOccupied)
    (bind _outactors (Collision|ComponentOverlapActors (Variables|Default|GetCollisionBox) (Transformation|GetActorTransform) (Utilities|Array|MakeArray "ObjectTypeQuery7") 0))
    (for _array_element _outactors
      (bind _asgrid_cell_bp (Utilities|Casting|CastToGridCellBP _array_element))
      (Variables|GridCellBP_C|SetIsBorderCell _asgrid_cell_bp false)
      (if (not (Variables|GridCellBP_C|GetIsOccupied _asgrid_cell_bp))
        (Variables|GridCellBP_C|SetIsBorderCell _asgrid_cell_bp true)
        (Utilities|Array|AddUnique (Variables|/Game/Assets/Fractions/FractionBaseBP.FractionBaseBP_C|GetBorderCellsArr (Variables|Default|GetOccupantFraction)) _asgrid_cell_bp)))
    (return)))

(fn SetResourceData
  (params (Plant%20Food :type Float%20%28single-precision%29) (Fowl :type Float%20%28single-precision%29) (Leather :type Float%20%28single-precision%29) (Fur :type Float%20%28single-precision%29) (Unique%20Source :type Name :default "None"))
  (bind _resourcelist (Variables|Default|GetResourceList))
  (Utilities|Map|Add _resourcelist "NewEnumerator0" Plant%20Food)
  (Utilities|Map|Add _resourcelist "NewEnumerator1" Fowl)
  (Utilities|Map|Add _resourcelist "NewEnumerator4" Leather)
  (Utilities|Map|Add _resourcelist "NewEnumerator5" Fur)
  (return))

(fn SetFowlEfficience
  (params (CellType :type CellTypeEnum%20Enum :default "NewEnumerator10"))
  (if (Math|Boolean|ORBoolean (Utilities|Enum|Equal(Enum) CellType "NewEnumerator5") (Utilities|Enum|Equal(Enum) CellType "NewEnumerator6") (Utilities|Enum|Equal(Enum) CellType "NewEnumerator12"))
    (LocalVariables|SetLocalFood 9e+01)
    (LocalVariables|SetLocalFur 1e+01)
    (LocalVariables|SetLocalLeather 6e+01)
    (elif (Math|Boolean|ORBoolean (Utilities|Enum|Equal(Enum) CellType "NewEnumerator7") (Utilities|Enum|Equal(Enum) CellType "NewEnumerator8") (Utilities|Enum|Equal(Enum) CellType "NewEnumerator11"))
      (LocalVariables|SetLocalFood 9e+01)
      (LocalVariables|SetLocalFur 6e+01)
      (LocalVariables|SetLocalLeather 1e+01)
      (elif (Math|Boolean|ORBoolean (Utilities|Enum|Equal(Enum) CellType "NewEnumerator3") (Utilities|Enum|Equal(Enum) CellType "NewEnumerator4") (Utilities|Enum|Equal(Enum) CellType "NewEnumerator13"))
        (LocalVariables|SetLocalFood 6e+01)
        (LocalVariables|SetLocalFur 1e+01)
        (LocalVariables|SetLocalLeather 1e+01)
        (else
          (LocalVariables|SetLocalFood 0.0)
          (LocalVariables|SetLocalFur 0.0)
          (LocalVariables|SetLocalLeather 0.0)))))
  (return (LocalVariables|GetLocalFood) (LocalVariables|GetLocalLeather) (LocalVariables|GetLocalFur)))

(fn ConstructionInitiate
  (params (CellBuilding :type Cell%20Building%20BP%20Class%20Reference))
  (bind _owningcity (Variables|Default|GetOwningCity))
  (bind _returnvalue (Game|SpawnActorfromClass CellBuilding (Math|Transform|MakeTransform (Transformation|GetActorLocation) "0, 0, 0" "1,1,1") "Undefined" 0 0))
  (bind _output_get (Variables|Default|SetCellBuildingRef _returnvalue))
  (bind _returnvalue_2 (AddComponent|AddCellBuildingSceneComponent false (Math|Transform|MakeTransform "0, 0, 0" "0, 0, 0" "1,1,1") _output_get))
  (bind _output_get_2 (Variables|Default|SetConstructionRef _returnvalue_2))
  (Variables|/Game/World/Grid/CellBuildingSceneComponent.CellBuildingSceneComponent_C|SetGridCellRef _output_get_2 self)
  (Default|SetConstructionMesh _output_get_2)
  (Variables|/Game/Assets/CellBuildings/CellBuildingBP.CellBuildingBP_C|SetCellRef (Variables|Default|GetCellBuildingRef) self)
  (Variables|/Game/Assets/CellBuildings/CellBuildingBP.CellBuildingBP_C|SetOwningCityRef (Variables|Default|GetCellBuildingRef) _owningcity)
  (Utilities|Array|Add (Variables|/Game/Assets/CityBaseBP.CityBaseBP_C|GetCellBuildingsArr _owningcity) (Variables|Default|GetCellBuildingRef)))