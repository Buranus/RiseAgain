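; City cell actor for the world grid that toggles its city's UI when clicked.
; On BeginPlay it runs the parent logic and flags itself as built through IsBuilded.
; Clicks check IsWidgetOpen on CityRef and call that object to open or close the city widget.
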(event EventBeginPlay
  (|CallParentFunction)
  (Variables|Default|SetIsBuilded true))

(event Collision|EventActorBeginOverlap
  (params (OtherActor :type Actor%20Object%20Reference))
  (|CallParentFunction OtherActor) ; This node is disabled and will not be called.\nDrag off pins to build functionality.
)

(event EventTick
  (params (DeltaSeconds :type Float%20%28single-precision%29))
  (|CallParentFunction DeltaSeconds) ; This node is disabled and will not be called.\nDrag off pins to build functionality.
)

(event MouseInput|EventActorOnClicked
  (params (ButtonPressed :type Key%20Structure))
  (bind _cityref (Variables|Default|GetCityRef))
  (if (Variables|/Game/Assets/CityBaseBP.CityBaseBP_C|GetIsWidgetOpen (Variables|Default|GetCityRef))
    (Default|CloseCityWidget _cityref)
    (else
      (Default|OpenCityWidget _cityref))))

(fn ConstructionScript
  (|CallParentFunction))