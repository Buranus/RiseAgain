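; PopulusBP represents a single citizen, deriving labor and food consumption from age group and DemographyRef standards.
; On BeginPlay it sets status flags: IsSuiJuris for the youngest groups, who eat half portions and get no labor assigned, and IsOutOfOrder for group 10, with quarter labor.
; GrowingUp increments age when the TurnBasedController's month matches the birth month, recomputes the age group and reruns that stat reset.
; The reset only raises flags, never clears them.
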(event Custom|CitizenStatsReset
  (CallFunction|SetSuiJuris)
  (CallFunction|SetLabor)
  (CallFunction|SetFoodConsumption))

(event EventBeginPlay
  (CallFunction|CitizenStatsReset))

(fn ConstructionScript)

(fn SetSuiJuris
  (if (<= (Variables|Default|GetCitizenAgeGroup) 2)
    (Variables|Default|SetIsSuiJuris true)
    (return)
    (elif (== (Variables|Default|GetCitizenAgeGroup) 10)
      (Variables|Default|SetIsOutOfOrder true)
      (return))))

(fn SetLabor
  (bind _demographyref (Variables|Default|GetDemographyRef))
  (bind _standardlabor (Variables|/Game/Assets/DemographyBP.DemographyBP_C|GetStandardLabor _demographyref))
  (if (not (Variables|Default|GetIsSuiJuris))
    (if (Variables|Default|GetIsOutOfOrder)
      (Variables|Default|SetLabor (/ _standardlabor 4.0))
      (return)
      (else
        (Variables|Default|SetLabor _standardlabor)
        (return)))))

(fn SetFoodConsumption
  (bind _demographyref (Variables|Default|GetDemographyRef))
  (bind _standardportion (Variables|/Game/Assets/DemographyBP.DemographyBP_C|GetStandardPortion _demographyref))
  (if (Variables|Default|GetIsSuiJuris)
    (Variables|Default|SetFoodConsumption (/ _standardportion 2.0))
    (return)
    (else
      (Variables|Default|SetFoodConsumption _standardportion)
      (return))))

(fn GrowingUp
  (bind _asturn_based_controller (Utilities|Casting|CastToTurnBasedController (Game|GetPlayerController 0)))
  (if (== (Variables|Default|GetMonthOfBirthday) (Variables|/Game/CoreBP/TurnBasedController.TurnBasedController_C|GetMonth _asturn_based_controller))
    (bind _result (Math|Integer|IncrementInt (Variables|Default|GetCitizenAge))
      (:%20%20
        (bind _currentgroup (Default|AgeGroupProcessing (Variables|Default|GetDemographyRef) _result))
        (Variables|Default|SetCitizenAgeGroup _currentgroup)
        (CallFunction|CitizenStatsReset)
        (return)))))