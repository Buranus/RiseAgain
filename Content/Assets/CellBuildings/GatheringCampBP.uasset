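; Gathering camp cell building that defines which resources it outputs, based on the cell it references.
; Its SetResourceOutput event calls the parent, then fills the ResourceOutput map from ResourcePool values.
; One specific cell prototype also gets an entry set to its pool value plus a flat bonus.
; It then prints every output key and value on screen, apparently for debugging.
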(event EventSetResourceOutput
  (bind _resourceoutput (Variables|Default|GetResourceOutput))
  (bind _resourceoutput_2 (Variables|Default|GetResourceOutput))
  (bind _resourcepool (Variables|Default|GetResourcePool))
  (|CallParentFunction)
  (Utilities|FlowControl|Sequence
    (:then_0
      (Utilities|Map|Add _resourceoutput "" (.Value (Utilities|Map|Find _resourcepool "")))
      (if (Utilities|Enum|Equal(Enum) (Variables|/Game/World/Grid/GridCellBP.GridCellBP_C|GetCellPrototypeEnum (Variables|Default|GetCellRef)) "NewEnumerator2")
        (Utilities|Map|Add _resourceoutput "NewEnumerator7" (+ (.Value (Utilities|Map|Find _resourcepool "NewEnumerator7")) 1e+01))))
    (:then_1
      (bind _keys (Utilities|Map|Keys _resourceoutput_2))
      (bind _values (Utilities|Map|Values _resourceoutput_2))
      (for (_array_element _array_index) _keys
        (Development|PrintString (Utilities|String|Append (Utilities|String|EnumtoString _array_element) "   " (Utilities|String|ToString(Float) (Utilities|Array|Get(acopy) _values _array_index))) true true "(R=0.000000,G=0.066501,B=0.237500,A=1.000000)" 5.0)))))

(fn ConstructionScript
  (|CallParentFunction))