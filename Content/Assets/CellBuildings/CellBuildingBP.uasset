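; CellBuildingBP is a building on a cell, owned by a city, that is built over several actions and then staffed.
; ConstructionProcess counts down the remaining actions, then flags completion, notifies its cell, calls GetWorkersAutomatically and runs the empty SetResourceOutput.
; GetWorkersAutomatically gathers the city's employable, unemployed population and fills worker slots at random.
; Each add and removal rolls its own random index, so they can hit different people.
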(event Collision|EventActorBeginOverlap
  (params (OtherActor :type Actor%20Object%20Reference)))

(event EventTick
  (params (DeltaSeconds :type Float%20%28single-precision%29)))

(fn ConstructionScript)

(fn SetResourceOutput
  (return))

(fn ConstructionProcess
  (Variables|Default|SetActionsForComplete (- (Variables|Default|GetActionsForComplete) 1))
  (if (<= (Variables|Default|GetActionsForComplete) 0)
    (Variables|Default|SetConstructionComplete true)
    (Default|ConstructionDone (Variables|Default|GetCellRef))
    (CallFunction|GetWorkersAutomatically)
    (CallFunction|SetResourceOutput)
    (return)
    (else
      (return))))

(fn GetWorkersAutomatically
  (bind _localpopulus (LocalVariables|GetLocalPopulus))
  (bind _returnvalue (Utilities|Array|Length _localpopulus))
  (bind _returnvalue_2 (Math|Random|RandomInteger _returnvalue))
  (bind _output (Utilities|Array|Get(acopy) _localpopulus _returnvalue_2))
  (for _array_element (Variables|/Game/Assets/CityBaseBP.CityBaseBP_C|GetPopulationArr (Variables|Default|GetOwningCityRef))
    (if (Variables|/Game/Assets/PopulusBP.PopulusBP_C|GetEmployable _array_element)
      (if (not (Variables|/Game/Assets/PopulusBP.PopulusBP_C|GetIsEmployed _array_element))
        (Utilities|Array|Add (LocalVariables|GetLocalPopulus) _array_element))))
  (for _index (range 1 (Variables|Default|GetWorkersMax))
    (Utilities|Array|Add (Variables|Default|GetCellBuildingWorkers) _output)
    (Utilities|Array|RemoveItem _localpopulus _output)
    (Utilities|Array|RemoveItem (Variables|/Game/Assets/CityBaseBP.CityBaseBP_C|GetPopulationArr (Variables|Default|GetOwningCityRef)) _output))
  (return))