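; HuntersCampBP is a cell building Blueprint for a hunter's camp that defines which resources it outputs.
; It extends the parent's SetResourceOutput event, copying values from its ResourcePool map into ResourceOutput.
; One resource type is always copied, and two others only when their pool value is above zero.
; BeginPlay, overlap and Tick are disabled stubs, and the construction script only calls the parent.
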(event EventBeginPlay
  (|CallParentFunction) ; This node is disabled and will not be called.\nDrag off pins to build functionality.
)

(event Collision|EventActorBeginOverlap
  (params (OtherActor :type Actor%20Object%20Reference))
  (|CallParentFunction OtherActor) ; This node is disabled and will not be called.\nDrag off pins to build functionality.
)

(event EventTick
  (params (DeltaSeconds :type Float%20%28single-precision%29))
  (|CallParentFunction DeltaSeconds) ; This node is disabled and will not be called.\nDrag off pins to build functionality.
)

(event EventSetResourceOutput
  (bind _resourcepool (Variables|Default|GetResourcePool))
  (bind _resourceoutput (Variables|Default|GetResourceOutput))
  (bind _value (Utilities|Map|Find _resourcepool "NewEnumerator5"))
  (bind _value_2 (Utilities|Map|Find _resourcepool "NewEnumerator4"))
  (|CallParentFunction)
  (Utilities|Map|Add _resourceoutput "NewEnumerator1" (.Value (Utilities|Map|Find _resourcepool "NewEnumerator1")))
  (Utilities|FlowControl|Sequence
    (:then_0
      (if (> _value_2 0.0)
        (Utilities|Map|Add _resourceoutput "NewEnumerator4" _value_2)))
    (:then_1
      (if (> _value 0.0)
        (Utilities|Map|Add _resourceoutput "NewEnumerator5" _value)))))

(fn ConstructionScript
  (|CallParentFunction))