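; Residential district building Blueprint for the city, a child class that configures itself from its DistrictStage.
; On BeginPlay, after the parent logic, it sets LaborCost from the stage, rising linearly per stage with a fixed override for one enum value.
; It then picks BuildingIcon from an icon array indexed by the same stage.
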(event EventBeginPlay
  (|CallParentFunction)
  (bind _laborcost (CallFunction|SetLaborCost (Variables|Default|GetDistrictStage)))
  (Variables|Default|SetLaborCost _laborcost)
  (CallFunction|SetIcon))

(fn ConstructionScript
  (|CallParentFunction))

(fn SetLaborCost
  (params (ProcessingStage :type ResidentDistrictEnum%20Enum :default "NewEnumerator0"))
  (if (Utilities|Enum|Equal(Enum) ProcessingStage "NewEnumerator7")
    (return 5e+03)
    (else
      (return (* (+ (Math|Conversions|ToFloat(Byte) ProcessingStage) 1.0) 1e+03)))))

(fn SetIcon
  (Variables|Default|SetBuildingIcon (Utilities|Array|Get(acopy) (Variables|Default|GetIconStagingArr) (Math|Conversions|ToInteger(Byte) (Variables|Default|GetDistrictStage))))
  (return))