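; Sabinian faction Blueprint, a child of a faction base that sets up the Sabinians' starting state in a strategy game.
; On BeginPlay it spawns the Sabinian dynasty actor and builds the faction's building list from a data table.
; Setting the capital generates its population through DemographyRef in age and gender cohort loops, then spawns the starting Chieftain's House and Dugouts Block from data table rows.
; Initial resources fill capital supply stocks and the dynasty's political capital.
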(event EventSettingCapital
  (params (CapitalRef :type City%20Cell%20BP%20Object%20Reference))
  (bind _capitalcityref (Variables|Default|GetCapitalCityRef))
  (bind _capitalcityref_2 (Variables|Default|GetCapitalCityRef))
  (bind _returnvalue (Transformation|GetActorLocation _capitalcityref_2))
  (bind _citybuildingsarr (Variables|/Game/Assets/CityBaseBP.CityBaseBP_C|GetCityBuildingsArr _capitalcityref))
  ;[1 1 1] "Setting Capital" Override
  (|CallParentFunction CapitalRef)
  (CallFunction|CapitalPopulationSabinian)
  (bind _returnvalue_2 (Utilities|GetDataTableRow "/Game/CoreBP/DataBases/CityBuildingSabiniansDT.CityBuildingSabiniansDT" "ChieftainsHouse")
    (:then
      (bind _returnvalue_3 (Game|SpawnActorfromClass (.CityBuildingClass (Utilities|Struct|BreakCityBuildingStruct _returnvalue_2)) (Math|Transform|MakeTransform _returnvalue "0, 0, 0" "1,1,1") "Undefined" 0 (.BuildingName (Utilities|Struct|BreakCityBuildingStruct _returnvalue_2)) (.LaborCost (Utilities|Struct|BreakCityBuildingStruct _returnvalue_2)) (.WorkersAmount (Utilities|Struct|BreakCityBuildingStruct _returnvalue_2)) (.BuildingIcon (Utilities|Struct|BreakCityBuildingStruct _returnvalue_2)) (.ResourcePrice (Utilities|Struct|BreakCityBuildingStruct _returnvalue_2)) (.SpecificPrice (Utilities|Struct|BreakCityBuildingStruct _returnvalue_2)) (.CityBuildingTags (Utilities|Struct|BreakCityBuildingStruct _returnvalue_2)) (.ResourceOutput (Utilities|Struct|BreakCityBuildingStruct _returnvalue_2)) (.SupplyOutput (Utilities|Struct|BreakCityBuildingStruct _returnvalue_2)) 0))
      (Utilities|Array|Add _citybuildingsarr _returnvalue_3)
      (bind _returnvalue_4 (Utilities|GetDataTableRow "/Game/CoreBP/DataBases/CityBuildingSabiniansDT.CityBuildingSabiniansDT" "DugoutsBlock")
        (:then
          (bind _returnvalue_5 (Game|SpawnActorfromClass (.CityBuildingClass (Utilities|Struct|BreakCityBuildingStruct _returnvalue_4)) (Math|Transform|MakeTransform _returnvalue "0, 0, 0" "1,1,1") "Undefined" 0 (.BuildingName (Utilities|Struct|BreakCityBuildingStruct _returnvalue_4)) (.LaborCost (Utilities|Struct|BreakCityBuildingStruct _returnvalue_4)) (.WorkersAmount (Utilities|Struct|BreakCityBuildingStruct _returnvalue_4)) (.BuildingIcon (Utilities|Struct|BreakCityBuildingStruct _returnvalue_4)) (.ResourcePrice (Utilities|Struct|BreakCityBuildingStruct _returnvalue_4)) (.SpecificPrice (Utilities|Struct|BreakCityBuildingStruct _returnvalue_4)) (.CityBuildingTags (Utilities|Struct|BreakCityBuildingStruct _returnvalue_4)) (.ResourceOutput (Utilities|Struct|BreakCityBuildingStruct _returnvalue_4)) (.SupplyOutput (Utilities|Struct|BreakCityBuildingStruct _returnvalue_4)) 0))
          (Utilities|Array|Add _citybuildingsarr _returnvalue_5)
          (Default|BuildingListInitialize (Variables|Default|GetCapitalCityRef)))))))

(event EventSetInitialResources
  (bind _resourcecounter (Variables|Default|GetResourceCounter))
  (bind _capitalcityref (Variables|Default|GetCapitalCityRef))
  (bind _citysuppliesstock (Variables|/Game/Assets/CityBaseBP.CityBaseBP_C|GetCitySuppliesStock _capitalcityref))
  ;[1 1 1] "Set Initial Resources" Override
  (Utilities|Map|Add _citysuppliesstock "NewEnumerator0" (.Value (Utilities|Map|Find _resourcecounter "Proviancy")))
  (Utilities|Map|Add _citysuppliesstock "NewEnumerator9" 1e+02)
  (Utilities|Map|Add _citysuppliesstock "NewEnumerator10" 1e+02)
  (Utilities|Map|Add _citysuppliesstock "NewEnumerator11" 2e+02)
  (Utilities|Map|Add _citysuppliesstock "NewEnumerator12" 5e+01)
  (Utilities|Map|Add _citysuppliesstock "NewEnumerator13" 5e+01)
  (Variables|/Game/Assets/Dynasties/DynastyBaseBP.DynastyBaseBP_C|SetPoliticalCapital (Variables|Default|GetDynastyRef) (Math|Float|Truncate (.Value (Utilities|Map|Find _resourcecounter "PoliticalCapital")))))

(event EventBeginPlay
  (|CallParentFunction)
  (bind _returnvalue (Game|SpawnActorfromClass "/Game/Assets/Dynasties/DynastySabinianBP.DynastySabinianBP_C" (Math|Transform|MakeTransform "0, 0, 0" "0, 0, 0" "1,1,1") "Undefined" 0 10 0))
  (Variables|Default|SetDynastyRef _returnvalue)
  (Variables|Default|SetFractionName "Sabinians")
  (CallFunction|MakeBuildingsArray (Variables|Default|GetBuildingListDT)))

(fn ConstructionScript
  (|CallParentFunction))

(fn CapitalPopulationSabinian
  (LocalVariables|SetLocalCounter 0)
  (while (< (LocalVariables|GetLocalCounter) (LocalVariables|GetLocalOlderMale))
    (bind _output_get (LocalVariables|SetLocalGender "NewEnumerator0"))
    (Default|NewPersonInitialize (Variables|Default|GetDemographyRef) (Math|Random|RandomIntegerinRange 41 55) _output_get (Utilities|Enum|ByteToEnumMonthEnum (Math|Conversions|ToByte(Integer) (Math|Random|RandomInteger 11))) (Variables|Default|GetCapitalCityRef))
    (Math|Integer|IncrementInt (LocalVariables|GetLocalCounter)))
  (LocalVariables|SetLocalCounter 0)
  (while (< (LocalVariables|GetLocalCounter) (LocalVariables|GetLocalOlderFemale))
    (bind _output_get_2 (LocalVariables|SetLocalGender "NewEnumerator1"))
    (Default|NewPersonInitialize (Variables|Default|GetDemographyRef) (Math|Random|RandomIntegerinRange 41 55) _output_get_2 (Utilities|Enum|ByteToEnumMonthEnum (Math|Conversions|ToByte(Integer) (Math|Random|RandomInteger 11))) (Variables|Default|GetCapitalCityRef))
    (Math|Integer|IncrementInt (LocalVariables|GetLocalCounter)))
  (LocalVariables|SetLocalCounter 0)
  (while (< (LocalVariables|GetLocalCounter) (LocalVariables|GetLocalOlderFuta))
    (bind _output_get_3 (LocalVariables|SetLocalGender "NewEnumerator2"))
    (Default|NewPersonInitialize (Variables|Default|GetDemographyRef) (Math|Random|RandomIntegerinRange 41 55) _output_get_3 (Utilities|Enum|ByteToEnumMonthEnum (Math|Conversions|ToByte(Integer) (Math|Random|RandomInteger 11))) (Variables|Default|GetCapitalCityRef))
    (Math|Integer|IncrementInt (LocalVariables|GetLocalCounter)))
  (LocalVariables|SetLocalCounter 0)
  (while (< (LocalVariables|GetLocalCounter) (LocalVariables|GetLocalAdultMale))
    (bind _output_get_4 (LocalVariables|SetLocalGender "NewEnumerator0"))
    (Default|NewPersonInitialize (Variables|Default|GetDemographyRef) (Math|Random|RandomIntegerinRange 13 40) _output_get_4 (Utilities|Enum|ByteToEnumMonthEnum (Math|Conversions|ToByte(Integer) (Math|Random|RandomInteger 11))) (Variables|Default|GetCapitalCityRef))
    (Math|Integer|IncrementInt (LocalVariables|GetLocalCounter)))
  (LocalVariables|SetLocalCounter 0)
  (while (< (LocalVariables|GetLocalCounter) (LocalVariables|GetLocalAdultFemale))
    (bind _output_get_5 (LocalVariables|SetLocalGender "NewEnumerator1"))
    (Default|NewPersonInitialize (Variables|Default|GetDemographyRef) (Math|Random|RandomIntegerinRange 13 40) _output_get_5 (Utilities|Enum|ByteToEnumMonthEnum (Math|Conversions|ToByte(Integer) (Math|Random|RandomInteger 11))) (Variables|Default|GetCapitalCityRef))
    (Math|Integer|IncrementInt (LocalVariables|GetLocalCounter)))
  (LocalVariables|SetLocalCounter 0)
  (while (< (LocalVariables|GetLocalCounter) (LocalVariables|GetLocalAdultFuta))
    (bind _output_get_6 (LocalVariables|SetLocalGender "NewEnumerator2"))
    (Default|NewPersonInitialize (Variables|Default|GetDemographyRef) (Math|Random|RandomIntegerinRange 13 40) _output_get_6 (Utilities|Enum|ByteToEnumMonthEnum (Math|Conversions|ToByte(Integer) (Math|Random|RandomInteger 11))) (Variables|Default|GetCapitalCityRef))
    (Math|Integer|IncrementInt (LocalVariables|GetLocalCounter)))
  (LocalVariables|SetLocalCounter 0)
  (while (< (LocalVariables|GetLocalCounter) (LocalVariables|GetLocalChildMale))
    (bind _output_get_7 (LocalVariables|SetLocalGender "NewEnumerator0"))
    (Default|NewPersonInitialize (Variables|Default|GetDemographyRef) (Math|Random|RandomIntegerinRange 2 12) _output_get_7 (Utilities|Enum|ByteToEnumMonthEnum (Math|Conversions|ToByte(Integer) (Math|Random|RandomInteger 11))) (Variables|Default|GetCapitalCityRef))
    (Math|Integer|IncrementInt (LocalVariables|GetLocalCounter)))
  (LocalVariables|SetLocalCounter 0)
  (while (< (LocalVariables|GetLocalCounter) (LocalVariables|GetLocalChildFemale))
    (bind _output_get_8 (LocalVariables|SetLocalGender "NewEnumerator1"))
    (Default|NewPersonInitialize (Variables|Default|GetDemographyRef) (Math|Random|RandomIntegerinRange 2 12) _output_get_8 (Utilities|Enum|ByteToEnumMonthEnum (Math|Conversions|ToByte(Integer) (Math|Random|RandomInteger 11))) (Variables|Default|GetCapitalCityRef))
    (Math|Integer|IncrementInt (LocalVariables|GetLocalCounter)))
  (LocalVariables|SetLocalCounter 0)
  (while (< (LocalVariables|GetLocalCounter) (LocalVariables|GetLocalChildFuta))
    (bind _output_get_9 (LocalVariables|SetLocalGender "NewEnumerator2"))
    (Default|NewPersonInitialize (Variables|Default|GetDemographyRef) (Math|Random|RandomIntegerinRange 2 12) _output_get_9 (Utilities|Enum|ByteToEnumMonthEnum (Math|Conversions|ToByte(Integer) (Math|Random|RandomInteger 11))) (Variables|Default|GetCapitalCityRef))
    (Math|Integer|IncrementInt (LocalVariables|GetLocalCounter)))
  (LocalVariables|SetLocalCounter 0)
  (while (< (LocalVariables|GetLocalCounter) (LocalVariables|GetLocalBabyMale))
    (bind _output_get_10 (LocalVariables|SetLocalGender "NewEnumerator0"))
    (Default|NewPersonInitialize (Variables|Default|GetDemographyRef) (Math|Random|RandomIntegerinRange 0 1) _output_get_10 (Utilities|Enum|ByteToEnumMonthEnum (Math|Conversions|ToByte(Integer) (Math|Random|RandomInteger 11))) (Variables|Default|GetCapitalCityRef))
    (Math|Integer|IncrementInt (LocalVariables|GetLocalCounter)))
  (LocalVariables|SetLocalCounter 0)
  (while (< (LocalVariables|GetLocalCounter) (LocalVariables|GetLocalBabyFemale))
    (bind _output_get_11 (LocalVariables|SetLocalGender "NewEnumerator1"))
    (Default|NewPersonInitialize (Variables|Default|GetDemographyRef) (Math|Random|RandomIntegerinRange 0 1) _output_get_11 (Utilities|Enum|ByteToEnumMonthEnum (Math|Conversions|ToByte(Integer) (Math|Random|RandomInteger 11))) (Variables|Default|GetCapitalCityRef))
    (Math|Integer|IncrementInt (LocalVariables|GetLocalCounter)))
  (return))