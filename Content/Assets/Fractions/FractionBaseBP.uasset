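; Base actor for a faction in a turn-based strategy game, owning its capital, cities, resources, action points and technology perks.
; It spawns resource, building and demography helpers, seeding a name-keyed resource counter from a DataTable.
; Turn start resets actions and updates cities and perk availability; turn end runs construction, feeding, harvesting and aging.
; Non-abstract resource totals are rebuilt from city stockpiles, which spending can drain.
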(event Custom|SettingCapital
  (params (CapitalRef :type City%20Cell%20BP%20Object%20Reference))
  (bind _output_get (Variables|References|SetCapitalCellRef CapitalRef))
  (Utilities|Array|Add (Variables|DataArrays|GetOwnedCellsArr) _output_get)
  (bind _returnvalue (Game|SpawnActorfromClass "/Game/Assets/CityBaseBP.CityBaseBP_C" (Math|Transform|MakeTransform (Transformation|GetActorLocation (Variables|References|GetCapitalCellRef)) "0, 0, 0" "1,1,1") "Undefined" 0 0))
  (bind _output_get_2 (Variables|References|SetCapitalCityRef _returnvalue))
  (Utilities|Array|AddUnique (Variables|DataArrays|GetCitiesArray) _output_get_2)
  (Variables|/Game/Assets/CityBaseBP.CityBaseBP_C|SetFractionRef (Variables|References|GetCapitalCityRef) self)
  (bind _output_get_3 (Variables|/Game/Assets/CityBaseBP.CityBaseBP_C|SetIsCapital (Variables|References|GetCapitalCityRef) true))
  (bind _output_get_4 (Variables|/Game/Assets/CityBaseBP.CityBaseBP_C|SetFullFunctioned (Variables|References|GetCapitalCityRef) _output_get_3))
  (Variables|/Game/Assets/CityBaseBP.CityBaseBP_C|SetConnectedWithCapital (Variables|References|GetCapitalCityRef) _output_get_4)
  (Variables|/Game/Assets/CityBaseBP.CityBaseBP_C|SetCityName (Variables|References|GetCapitalCityRef) "Imperion")
  (Variables|/Game/Assets/CityBaseBP.CityBaseBP_C|SetCityCellRef (Variables|References|GetCapitalCityRef) (Variables|References|GetCapitalCellRef))
  (Variables|/Game/World/Grid/CityCellBP.CityCellBP_C|SetCityRef (Variables|References|GetCapitalCellRef) (Variables|References|GetCapitalCityRef))
  (Variables|/Game/World/Grid/GridCellBP.GridCellBP_C|SetIsOccupied (Variables|References|GetCapitalCellRef) true)
  (Variables|/Game/World/Grid/GridCellBP.GridCellBP_C|SetOccupantFraction (Variables|References|GetCapitalCellRef) self)
  (CallFunction|SetInitialResources))

(event Custom|TurnBegan
  (Utilities|FlowControl|Sequence
    (:then_0
      (CallFunction|ActionsCountZeroing)
      (for _array_element (Variables|DataArrays|GetCitiesArray)
        (Default|GetLaborPerTurn _array_element)
        (Default|CheckPrerequisites _array_element)
        ;[1 1 1] Debug
        (for _array_element_2 (Variables|/Game/Assets/CityBaseBP.CityBaseBP_C|GetPrerequisitesList _array_element)
          (Development|PrintString (Utilities|String|ToString(Name) _array_element_2) true true "(R=0.000000,G=0.057573,B=0.641667,A=1.000000)" 1e+01))))
    (:then_1
      (CallFunction|UpdatePerkTrees))))

(event Custom|TurnEnded
  (Utilities|FlowControl|Sequence
    (:then_0
      (for _array_element (Variables|DataArrays|GetCitiesArray)
        (Default|ConstructionUpdate _array_element)
        (Default|CitizensFeeding _array_element)))
    (:then_1
      (CallFunction|CollectResources)
      (CallFunction|PopulusAgeUpdate)
      (CallFunction|RecheckResourceCounter))))

(event EventBeginPlay
  (bind _returnvalue (Transformation|GetActorLocation))
  (CallFunction|SetResourceNames)
  (bind _returnvalue_2 (Game|SpawnActorfromClass "/Game/Assets/CellBuildings/CellBuildingBP.CellBuildingBP_C" (Math|Transform|MakeTransform _returnvalue "0, 0, 0" "1,1,1") "Undefined" 0 0))
  (bind _output_get (Variables|References|SetCellBuildingRef _returnvalue_2))
  (Variables|/Game/Assets/CellBuildings/CellBuildingBP.CellBuildingBP_C|SetResourceBaseRef _output_get (Variables|References|GetResourceBaseRef))
  (bind _returnvalue_3 (Game|SpawnActorfromClass "/Game/Assets/DemographyBP.DemographyBP_C" (Math|Transform|MakeTransform _returnvalue "0, 0, 0" "1,1,1") "Undefined" 0 0))
  (Variables|References|SetDemographyRef _returnvalue_3))

(fn ConstructionScript)

(fn TakeAnAction
  (if (> (Variables|ActionMechanics|GetActionsRemained) 0)
    (Math|Integer|DecrementInt (Variables|ActionMechanics|GetActionsRemained)
      (:%20%20
        (return true)))
    (else
      (return false))))

(fn ActionsCountZeroing
  (Variables|ActionMechanics|SetActionsRemained (/ (Variables|ActionMechanics|GetDaysPerTurn) (Variables|/Game/Assets/Dynasties/DynastyBaseBP.DynastyBaseBP_C|GetRulerDaysPerAct (Variables|References|GetDynastyRef))))
  (return))

(fn SetResourceNames
  (bind _returnvalue (Transformation|GetActorTransform))
  (bind _returnvalue_2 (Transformation|GetActorTransform))
  (bind _resourcearr (Variables|GlobalResources|GetResourceArr))
  (bind _returnvalue_3 (Game|SpawnActorfromClass "/Game/Assets/Resources/ResourceBaseBP.ResourceBaseBP_C" (Transformation|GetActorTransform) "Undefined" 0 0 "None" 0))
  (Variables|References|SetResourceBaseRef _returnvalue_3)
  (Utilities|FlowControl|Sequence
    (:then_0
      (bind _returnvalue_4 (Utilities|GetDataTableRow "/Game/CoreBP/DataBases/ResourcesData/SourceButtonsDT.SourceButtonsDT" "PoliticalCapital")
        (:then
          (Utilities|Map|Add (Variables|Default|GetResourceCounter) (.SourceName (Utilities|Struct|BreakSourceButtonStruct _returnvalue_4)) (Math|Conversions|ToFloat(Integer) (.SourceQuantity (Utilities|Struct|BreakSourceButtonStruct _returnvalue_4))))
          (bind _returnvalue_5 (Game|SpawnActorfromClass (.SourceActorRef (Utilities|Struct|BreakSourceButtonStruct _returnvalue_4)) _returnvalue_2 "AlwaysSpawn" 0 (.SourceImage (Utilities|Struct|BreakSourceButtonStruct _returnvalue_4)) (.SourceName (Utilities|Struct|BreakSourceButtonStruct _returnvalue_4)) 0))
          (bind _output_get (Variables|GlobalResources|SetPoliticalCapitalRef _returnvalue_5))
          (Utilities|Array|Add _resourcearr _output_get)
          (bind _returnvalue_6 (Utilities|GetDataTableRow "/Game/CoreBP/DataBases/ResourcesData/SourceButtonsDT.SourceButtonsDT" "Proviancy")
            (:then
              (Utilities|Map|Add (Variables|Default|GetResourceCounter) (.SourceName (Utilities|Struct|BreakSourceButtonStruct _returnvalue_6)) (Math|Conversions|ToFloat(Integer) (.SourceQuantity (Utilities|Struct|BreakSourceButtonStruct _returnvalue_6))))
              (bind _returnvalue_7 (Game|SpawnActorfromClass (.SourceActorRef (Utilities|Struct|BreakSourceButtonStruct _returnvalue_6)) _returnvalue "AlwaysSpawn" 0 (.SourceImage (Utilities|Struct|BreakSourceButtonStruct _returnvalue_6)) (.SourceName (Utilities|Struct|BreakSourceButtonStruct _returnvalue_6)) 0))
              (bind _output_get_2 (Variables|GlobalResources|SetProviancyRef _returnvalue_7))
              (Utilities|Array|Add _resourcearr _output_get_2))))))
    (:then_1
      (bind _returnvalue_8 (Utilities|GetDataTableRow "/Game/CoreBP/DataBases/ResourcesData/SourceButtonsDT.SourceButtonsDT" "Wood")
        (:then
          (Utilities|Map|Add (Variables|Default|GetResourceCounter) (.SourceName (Utilities|Struct|BreakSourceButtonStruct _returnvalue_8)) (Math|Conversions|ToFloat(Integer) (.SourceQuantity (Utilities|Struct|BreakSourceButtonStruct _returnvalue_8))))
          (bind _returnvalue_9 (Game|SpawnActorfromClass (.SourceActorRef (Utilities|Struct|BreakSourceButtonStruct _returnvalue_8)) _returnvalue_2 "AlwaysSpawn" 0 (.SourceImage (Utilities|Struct|BreakSourceButtonStruct _returnvalue_8)) "None" 0))
          (bind _output_get_3 (Variables|GlobalResources|SetWoodResourceRef _returnvalue_9))
          (Utilities|Array|Add _resourcearr _output_get_3)
          (bind _returnvalue_10 (Utilities|GetDataTableRow "/Game/CoreBP/DataBases/ResourcesData/SourceButtonsDT.SourceButtonsDT" "Stone")
            (:then
              (Utilities|Map|Add (Variables|Default|GetResourceCounter) (.SourceName (Utilities|Struct|BreakSourceButtonStruct _returnvalue_10)) (Math|Conversions|ToFloat(Integer) (.SourceQuantity (Utilities|Struct|BreakSourceButtonStruct _returnvalue_10))))
              (bind _returnvalue_11 (Game|SpawnActorfromClass (.SourceActorRef (Utilities|Struct|BreakSourceButtonStruct _returnvalue_10)) _returnvalue "AlwaysSpawn" 0 (.SourceImage (Utilities|Struct|BreakSourceButtonStruct _returnvalue_10)) "None" 0))
              (bind _output_get_4 (Variables|GlobalResources|SetStoneResourceRef _returnvalue_11))
              (Utilities|Array|Add _resourcearr _output_get_4))))))
    (:then_2
      (bind _returnvalue_12 (Utilities|GetDataTableRow "/Game/CoreBP/DataBases/ResourcesData/SourceButtonsDT.SourceButtonsDT" "Knowledge")
        (:then
          (Utilities|Map|Add (Variables|Default|GetResourceCounter) (.SourceName (Utilities|Struct|BreakSourceButtonStruct _returnvalue_12)) (Math|Conversions|ToFloat(Integer) (.SourceQuantity (Utilities|Struct|BreakSourceButtonStruct _returnvalue_12))))
          (bind _returnvalue_13 (Game|SpawnActorfromClass (.SourceActorRef (Utilities|Struct|BreakSourceButtonStruct _returnvalue_12)) (Transformation|GetActorTransform) "AlwaysSpawn" 0 (.SourceImage (Utilities|Struct|BreakSourceButtonStruct _returnvalue_12)) "None" 0))
          (bind _output_get_5 (Variables|GlobalResources|SetKnowledgeRef _returnvalue_13))
          (Utilities|Array|Add _resourcearr _output_get_5))))
    (:then_3
      (return))))

(fn GetStartRegion
  (bind _asturn_based_controller (Utilities|Casting|CastToTurnBasedController (Game|GetPlayerController 0)))
  (Default|OccupyCell (Utilities|Array|Get(acopy) (Variables|/Game/CoreBP/TurnBasedController.TurnBasedController_C|GetGridMapArr _asturn_based_controller) (- (Utilities|Array|FindItem (Variables|/Game/CoreBP/TurnBasedController.TurnBasedController_C|GetGridMapArr _asturn_based_controller) (Variables|References|GetCapitalCellRef)) 16)))
  (Default|OccupyCell (Utilities|Array|Get(acopy) (Variables|/Game/CoreBP/TurnBasedController.TurnBasedController_C|GetGridMapArr _asturn_based_controller) (- (Utilities|Array|FindItem (Variables|/Game/CoreBP/TurnBasedController.TurnBasedController_C|GetGridMapArr _asturn_based_controller) (Variables|References|GetCapitalCellRef)) 15)))
  (Default|OccupyCell (Utilities|Array|Get(acopy) (Variables|/Game/CoreBP/TurnBasedController.TurnBasedController_C|GetGridMapArr _asturn_based_controller) (- (Utilities|Array|FindItem (Variables|/Game/CoreBP/TurnBasedController.TurnBasedController_C|GetGridMapArr _asturn_based_controller) (Variables|References|GetCapitalCellRef)) 14)))
  (Default|OccupyCell (Utilities|Array|Get(acopy) (Variables|/Game/CoreBP/TurnBasedController.TurnBasedController_C|GetGridMapArr _asturn_based_controller) (- (Utilities|Array|FindItem (Variables|/Game/CoreBP/TurnBasedController.TurnBasedController_C|GetGridMapArr _asturn_based_controller) (Variables|References|GetCapitalCellRef)) 1)))
  (Default|OccupyCell (Utilities|Array|Get(acopy) (Variables|/Game/CoreBP/TurnBasedController.TurnBasedController_C|GetGridMapArr _asturn_based_controller) (+ (Utilities|Array|FindItem (Variables|/Game/CoreBP/TurnBasedController.TurnBasedController_C|GetGridMapArr _asturn_based_controller) (Variables|References|GetCapitalCellRef)) 1)))
  (Default|OccupyCell (Utilities|Array|Get(acopy) (Variables|/Game/CoreBP/TurnBasedController.TurnBasedController_C|GetGridMapArr _asturn_based_controller) (+ (Utilities|Array|FindItem (Variables|/Game/CoreBP/TurnBasedController.TurnBasedController_C|GetGridMapArr _asturn_based_controller) (Variables|References|GetCapitalCellRef)) 14)))
  (Default|OccupyCell (Utilities|Array|Get(acopy) (Variables|/Game/CoreBP/TurnBasedController.TurnBasedController_C|GetGridMapArr _asturn_based_controller) (+ (Utilities|Array|FindItem (Variables|/Game/CoreBP/TurnBasedController.TurnBasedController_C|GetGridMapArr _asturn_based_controller) (Variables|References|GetCapitalCellRef)) 15)))
  (Default|OccupyCell (Utilities|Array|Get(acopy) (Variables|/Game/CoreBP/TurnBasedController.TurnBasedController_C|GetGridMapArr _asturn_based_controller) (+ (Utilities|Array|FindItem (Variables|/Game/CoreBP/TurnBasedController.TurnBasedController_C|GetGridMapArr _asturn_based_controller) (Variables|References|GetCapitalCellRef)) 16)))
  (Default|VerifyCityZone (Variables|References|GetCapitalCityRef))
  (return))

(fn CollectResources
  (bind _resourcecounter (Variables|Default|GetResourceCounter))
  (for _array_element (Variables|DataArrays|GetCitiesArray)
    (bind _abstractsoutput (Default|HarvestInternalResources _array_element))
    (bind _monthincome (Default|HarvestingSupplies _array_element))
    (Utilities|FlowControl|Sequence
      (:then_0
        (LocalVariables|SetLocalMonthIncome _resourcecounter)
        (Utilities|Map|Clear _resourcecounter)
        (bind _output_get (LocalVariables|SetLocalInternalResources _abstractsoutput)))
      (:then_1
        (bind _returnvalue (Utilities|GetDataTableRow "/Game/CoreBP/DataBases/ResourcesData/SourceButtonsDT.SourceButtonsDT" "PoliticalCapital")
          (:then
            (if (.ReturnValue (Utilities|Map|Find (LocalVariables|GetLocalMonthIncome) (.SourceName (Utilities|Struct|BreakSourceButtonStruct _returnvalue))))
              (Utilities|Map|Add (Variables|Default|GetResourceCounter) (.SourceName (Utilities|Struct|BreakSourceButtonStruct _returnvalue)) (+ (.Value (Utilities|Map|Find (LocalVariables|GetLocalMonthIncome) (.SourceName (Utilities|Struct|BreakSourceButtonStruct _returnvalue)))) (.Value (Utilities|Map|Find _output_get "PoliticalCapital"))))))))
      (:then_2
        (bind _returnvalue_2 (Utilities|GetDataTableRow "/Game/CoreBP/DataBases/ResourcesData/SourceButtonsDT.SourceButtonsDT" "Treasury")
          (:then
            (if (.ReturnValue (Utilities|Map|Find (LocalVariables|GetLocalMonthIncome) (.SourceName (Utilities|Struct|BreakSourceButtonStruct _returnvalue_2))))
              (Utilities|Map|Add (Variables|Default|GetResourceCounter) (.SourceName (Utilities|Struct|BreakSourceButtonStruct _returnvalue_2)) (.Value (Utilities|Map|Find (LocalVariables|GetLocalMonthIncome) (.SourceName (Utilities|Struct|BreakSourceButtonStruct _returnvalue_2)))))))))
      (:then_3
        (bind _returnvalue_3 (Utilities|GetDataTableRow "/Game/CoreBP/DataBases/ResourcesData/SourceButtonsDT.SourceButtonsDT" "Proviancy")
          (:then
            (if (.ReturnValue (Utilities|Map|Find (LocalVariables|GetLocalMonthIncome) (.SourceName (Utilities|Struct|BreakSourceButtonStruct _returnvalue_3))))
              (Utilities|Map|Add (Variables|Default|GetResourceCounter) (.SourceName (Utilities|Struct|BreakSourceButtonStruct _returnvalue_3)) (+ (.Value (Utilities|Map|Find (LocalVariables|GetLocalMonthIncome) (.SourceName (Utilities|Struct|BreakSourceButtonStruct _returnvalue_3)))) (+ (.Value (Utilities|Map|Find _monthincome "")) (.Value (Utilities|Map|Find _monthincome "NewEnumerator1")) (.Value (Utilities|Map|Find _monthincome "NewEnumerator2")) (.Value (Utilities|Map|Find _monthincome "NewEnumerator3")) (.Value (Utilities|Map|Find _monthincome "NewEnumerator6")))))))))
      (:then_4
        (bind _returnvalue_4 (Utilities|GetDataTableRow "/Game/CoreBP/DataBases/ResourcesData/SourceButtonsDT.SourceButtonsDT" "Wood")
          (:then
            (if (.ReturnValue (Utilities|Map|Find (LocalVariables|GetLocalMonthIncome) (.SourceName (Utilities|Struct|BreakSourceButtonStruct _returnvalue_4))))
              (Utilities|Map|Add (Variables|Default|GetResourceCounter) (.SourceName (Utilities|Struct|BreakSourceButtonStruct _returnvalue_4)) (+ (.Value (Utilities|Map|Find (LocalVariables|GetLocalMonthIncome) (.SourceName (Utilities|Struct|BreakSourceButtonStruct _returnvalue_4)))) (.Value (Utilities|Map|Find _monthincome "NewEnumerator7"))))))))
      (:then_5
        (bind _returnvalue_5 (Utilities|GetDataTableRow "/Game/CoreBP/DataBases/ResourcesData/SourceButtonsDT.SourceButtonsDT" "Stone")
          (:then
            (if (.ReturnValue (Utilities|Map|Find (LocalVariables|GetLocalMonthIncome) (.SourceName (Utilities|Struct|BreakSourceButtonStruct _returnvalue_5))))
              (Utilities|Map|Add (Variables|Default|GetResourceCounter) (.SourceName (Utilities|Struct|BreakSourceButtonStruct _returnvalue_5)) (+ (.Value (Utilities|Map|Find (LocalVariables|GetLocalMonthIncome) (.SourceName (Utilities|Struct|BreakSourceButtonStruct _returnvalue_5)))) (.Value (Utilities|Map|Find _monthincome "NewEnumerator8"))))))))
      (:then_6
        (bind _returnvalue_6 (Utilities|GetDataTableRow "/Game/CoreBP/DataBases/ResourcesData/SourceButtonsDT.SourceButtonsDT" "Knowledge")
          (:then
            (if (.ReturnValue (Utilities|Map|Find (LocalVariables|GetLocalMonthIncome) (.SourceName (Utilities|Struct|BreakSourceButtonStruct _returnvalue_6))))
              (Utilities|Map|Add (Variables|Default|GetResourceCounter) (.SourceName (Utilities|Struct|BreakSourceButtonStruct _returnvalue_6)) (+ (.Value (Utilities|Map|Find (LocalVariables|GetLocalMonthIncome) (.SourceName (Utilities|Struct|BreakSourceButtonStruct _returnvalue_6)))) (.Value (Utilities|Map|Find _output_get "Knowledge"))))))))))
  (return))

(fn SetInitialResources
  (return))

(fn PopulusAgeUpdate
  (bind _asturn_based_controller (Utilities|Casting|CastToTurnBasedController (Game|GetPlayerController 0)))
  (LocalVariables|SetLocalMonth (Variables|/Game/CoreBP/TurnBasedController.TurnBasedController_C|GetMonthEnum _asturn_based_controller))
  (for _array_element (Variables|DataArrays|GetCitiesArray)
    (for _array_element_2 (Variables|/Game/Assets/CityBaseBP.CityBaseBP_C|GetPopulationArr _array_element)
      (Default|GrowingUp _array_element_2)))
  (return))

(fn CheckSolvency
  (params (PurchasePrice :type Map%20of%20SourcesEnum%20Enums%20to%20Integers :default "NewEnumerator6"))
  (bind _keys (Utilities|Map|Keys PurchasePrice))
  (for _array_element _keys
    (if (>= (.Value (Utilities|Map|Find (Variables|Default|GetResourceCounter) (Utilities|String|StringToName (Utilities|String|EnumtoString _array_element)))) (Math|Conversions|ToFloat(Integer) (.Value (Utilities|Map|Find PurchasePrice _array_element))))
      (Utilities|Map|Add (LocalVariables|GetLocalMap) (Utilities|String|StringToName (Utilities|String|EnumtoString _array_element)) (Math|Conversions|ToFloat(Integer) (.Value (Utilities|Map|Find PurchasePrice _array_element))))
      (else
        (return false 0))))
  (return true (LocalVariables|GetLocalMap)))

(fn ExpencesProcessing
  (params (ProcessedCity :type City%20Base%20BP%20Object%20Reference) (Expenses :type Map%20of%20Names%20to%20Float%20%28single-precision%29s))
  (bind _resourcecounter (Variables|Default|GetResourceCounter))
  (bind _citysuppliesstock (Variables|/Game/Assets/CityBaseBP.CityBaseBP_C|GetCitySuppliesStock ProcessedCity))
  (bind _localsupply (LocalVariables|GetLocalSupply))
  (LocalVariables|SetLocalStock _resourcecounter)
  (Utilities|Map|Clear _resourcecounter)
  (bind _output_get (LocalVariables|SetLocalCost Expenses))
  (bind _keys (Utilities|Map|Keys (LocalVariables|GetLocalStock)))
  (for _array_element _keys
    (if (.ReturnValue (Utilities|Map|Find _output_get _array_element))
      (bind _output_get_2 (LocalVariables|SetLocalName _array_element))
      (bind _output_get_3 (LocalVariables|SetLocalAmount (.Value (Utilities|Map|Find _output_get _array_element))))
      (Utilities|Map|Add (Variables|Default|GetResourceCounter) (LocalVariables|GetLocalName) (- (.Value (Utilities|Map|Find (LocalVariables|GetLocalStock) _output_get_2)) _output_get_3))
      (for _array_element_2 (Variables|GlobalResources|GetResourceArr)
        (if (Utilities|Name|Equal(Name) (LocalVariables|GetLocalName) (Variables|/Game/Assets/Resources/ResourceBaseBP.ResourceBaseBP_C|GetName _array_element_2))
          (bind _keys_2 (Utilities|Map|Keys _citysuppliesstock))
          (bind _array_element_3 (Utilities|Array|ForEachLoopwithBreak _keys_2 :!label _label)
            (:LoopBody
              (if (> (LocalVariables|GetLocalAmount) 0.0)
                (if (Utilities|Array|ContainsItem (Variables|/Game/Assets/Resources/ResourceBaseBP.ResourceBaseBP_C|GetIncludedResources _array_element_2) _array_element_3)
                  (if (< (LocalVariables|GetLocalAmount) (.Value (Utilities|Map|Find _citysuppliesstock _array_element_3)))
                    (Utilities|Map|Add (LocalVariables|GetLocalSupply) _array_element_3 (- (.Value (Utilities|Map|Find _citysuppliesstock _array_element_3)) (LocalVariables|GetLocalAmount)))
                    (LocalVariables|SetLocalAmount 0.0)
                    (Utilities|Map|Remove (Variables|/Game/Assets/CityBaseBP.CityBaseBP_C|GetCitySuppliesStock ProcessedCity) _array_element_3)
                    (else
                      (LocalVariables|SetLocalAmount (- (LocalVariables|GetLocalAmount) (.Value (Utilities|Map|Find _citysuppliesstock _array_element_3))))
                      (Utilities|Map|Remove _citysuppliesstock _array_element_3))))
                (else
                  (goto _label Break))))
            (:Completed
              (bind _keys_3 (Utilities|Map|Keys _localsupply))
              (for _array_element_4 _keys_3
                (Utilities|Map|Add (Variables|/Game/Assets/CityBaseBP.CityBaseBP_C|GetCitySuppliesStock ProcessedCity) _array_element_4 (.Value (Utilities|Map|Find _localsupply _array_element_4))))))))
      (else
        (Utilities|Map|Add (Variables|Default|GetResourceCounter) _array_element (.Value (Utilities|Map|Find (LocalVariables|GetLocalStock) _array_element))))))
  (Default|UpdateStatusBar (Variables|/Game/UI-UX/Widgets/MainUI.MainUI_C|GetStatusBar (Variables|/Game/CoreBP/TurnBasedController.TurnBasedController_C|GetMainWidgetRef (Variables|References|GetTBControllerRef))))
  (return))

(fn RecheckResourceCounter
  (bind _resourcecounter (Variables|Default|GetResourceCounter))
  (for _array_element (Variables|GlobalResources|GetResourceArr)
    (LocalVariables|SetLocalResource 0.0)
    (Utilities|Casting|CastToAbstractResourcesBP _array_element
      (:CastFailed
        (for _array_element_2 (Variables|DataArrays|GetCitiesArray)
          (for _array_element_3 (Variables|/Game/Assets/Resources/ResourceBaseBP.ResourceBaseBP_C|GetIncludedResources _array_element)
            (LocalVariables|SetLocalResource (+ (.Value (Utilities|Map|Find (Variables|/Game/Assets/CityBaseBP.CityBaseBP_C|GetCitySuppliesStock _array_element_2) _array_element_3)) (LocalVariables|GetLocalResource)))))
        (Utilities|Map|Remove _resourcecounter (Variables|/Game/Assets/Resources/ResourceBaseBP.ResourceBaseBP_C|GetName _array_element))
        (Utilities|Map|Add _resourcecounter (Variables|/Game/Assets/Resources/ResourceBaseBP.ResourceBaseBP_C|GetName _array_element) (LocalVariables|GetLocalResource)))))
  (return))

(fn MakeBuildingsArray
  (params (BuildingsList :type Data%20Table%20Object%20Reference))
  (bind _outrownames (DataTable|GetDataTableRowNames BuildingsList))
  (for _array_element _outrownames
    (Utilities|Array|Add (Variables|DataArrays|GetBuildNameList) _array_element))
  (return))

(fn SetWayOfDevelopment
  (params (TechnologyTree :type User%20Widget%20Class%20Reference))
  (bind _tbcontrollerref (Variables|References|GetTBControllerRef))
  (bind _mainwidgetref (Variables|/Game/CoreBP/TurnBasedController.TurnBasedController_C|GetMainWidgetRef _tbcontrollerref))
  (bind _returnvalue (UserInterface|CreateWidget TechnologyTree))
  (bind _output_get (Variables|/Game/UI-UX/Widgets/MainUI.MainUI_C|SetPerkTreeRef _mainwidgetref _returnvalue))
  (Widget|Panel|AddChild (Variables|/Game/UI-UX/Widgets/MainUI.MainUI_C|GetStateWindowBorder _mainwidgetref) _output_get)
  (return))

(fn PerkPurchasing
  (params (Perk :type Technology%20Widget%20Object%20Reference))
  (bind _technologystruct (Variables|/Game/UI-UX/Widgets/TechnologyWidget.TechnologyWidget_C|GetTechnologyStruct Perk))
  (bind (_technologyicon _technology _technologyclass _prerequisitestech _resourcecost) (Utilities|Struct|BreakTechnologiesStruct _technologystruct))
  (bind (_checkpassed _pricelist) (CallFunction|CheckSolvency _resourcecost))
  (if _checkpassed
    (bind _actionmade (CallFunction|TakeAnAction))
    (if _actionmade
      (CallFunction|ExpencesProcessing 0 _pricelist)
      (Utilities|Array|Add (Variables|Default|GetActivatedPerksArr) _technology)
      (Variables|/Game/UI-UX/Widgets/TechnologyWidget.TechnologyWidget_C|SetIsActive Perk true)
      (Default|ColorMarking Perk)
      (return)
      (else
        (Development|PrintString "No action points" true true "(R=1.000000,G=0.000000,B=0.006995,A=1.000000)" 1e+01)))
    (else
      (Development|PrintString "You have no resources for this" true true "(R=1.000000,G=0.000000,B=0.006995,A=1.000000)" 1e+01))))

(fn UpdatePerkTrees
  (for _array_element (Variables|Default|GetTechnologyArr)
    (if (not (Variables|/Game/UI-UX/Widgets/TechnologyWidget.TechnologyWidget_C|GetIsActive _array_element))
      (if (not (Variables|/Game/UI-UX/Widgets/TechnologyWidget.TechnologyWidget_C|GetIsAvailable _array_element))
        (bind _array_element_2 (Utilities|Array|ForEachLoopwithBreak (.PrerequisitesTech (Utilities|Struct|BreakTechnologiesStruct (Variables|/Game/UI-UX/Widgets/TechnologyWidget.TechnologyWidget_C|GetTechnologyStruct _array_element))) :!label _label)
          (:LoopBody
            (if (Utilities|Array|ContainsItem (Variables|Default|GetActivatedPerksArr) _array_element_2)
              (Variables|/Game/UI-UX/Widgets/TechnologyWidget.TechnologyWidget_C|SetIsAvailable _array_element true)
              (else
                (Variables|/Game/UI-UX/Widgets/TechnologyWidget.TechnologyWidget_C|SetIsAvailable _array_element false)
                (goto _label Break))))
          (:Completed
            (Default|ColorMarking _array_element))))))
  (return))