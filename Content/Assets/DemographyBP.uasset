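; Demography actor that creates citizens for cities and classifies them by age.
; NewPersonInitialize spawns a PopulusBP at the City's transform with age, gender, birth month, age group and employability, then registers it with the City.
; AgeGroupProcessing checks membership in per-group age collections, defaulting to the last group, and SetWorkingCapacity marks groups in AgeGroupVeto as unemployable.
; The event graph holds only disabled events and unconnected age-set editing nodes.
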(event EventBeginPlay)

(event Collision|EventActorBeginOverlap
  (params (OtherActor :type Actor%20Object%20Reference)))

(event EventTick
  (params (DeltaSeconds :type Float%20%28single-precision%29)))

(fn ConstructionScript)

(fn AgeGroupProcessing
  (params (CurrentAge :type Integer))
  (bind _agegroups (Variables|Default|GetAgeGroups))
  (bind (_baby _kid _child _teenage _juvenile _young _adult _mature _aged) (Utilities|Struct|BreakPopulusAgeStruct _agegroups))
  (Variables|Default|SetCurrentAge CurrentAge)
  (if (Utilities|Set|Contains _baby (Variables|Default|GetCurrentAge))
    (bind _output_get (Variables|Default|SetCurrentAgeGroup "NewEnumerator0"))
    (return _output_get)
    (elif (Utilities|Set|Contains _kid (Variables|Default|GetCurrentAge))
      (bind _output_get_2 (Variables|Default|SetCurrentAgeGroup "NewEnumerator1"))
      (return _output_get_2)
      (elif (Utilities|Set|Contains _child (Variables|Default|GetCurrentAge))
        (bind _output_get_3 (Variables|Default|SetCurrentAgeGroup "NewEnumerator2"))
        (return _output_get_3)
        (elif (Utilities|Set|Contains _teenage (Variables|Default|GetCurrentAge))
          (bind _output_get_4 (Variables|Default|SetCurrentAgeGroup "NewEnumerator3"))
          (return _output_get_4)
          (elif (Utilities|Set|Contains _juvenile (Variables|Default|GetCurrentAge))
            (bind _output_get_5 (Variables|Default|SetCurrentAgeGroup "NewEnumerator4"))
            (return _output_get_5)
            (elif (Utilities|Set|Contains _young (Variables|Default|GetCurrentAge))
              (bind _output_get_6 (Variables|Default|SetCurrentAgeGroup "NewEnumerator5"))
              (return _output_get_6)
              (elif (Utilities|Set|Contains _adult (Variables|Default|GetCurrentAge))
                (bind _output_get_7 (Variables|Default|SetCurrentAgeGroup "NewEnumerator6"))
                (return _output_get_7)
                (elif (Utilities|Set|Contains _mature (Variables|Default|GetCurrentAge))
                  (bind _output_get_8 (Variables|Default|SetCurrentAgeGroup "NewEnumerator7"))
                  (return _output_get_8)
                  (elif (Utilities|Set|Contains _aged (Variables|Default|GetCurrentAge))
                    (bind _output_get_9 (Variables|Default|SetCurrentAgeGroup "NewEnumerator8"))
                    (return _output_get_9)
                    (else
                      (bind _output_get_10 (Variables|Default|SetCurrentAgeGroup "NewEnumerator9"))
                      (return _output_get_10))))))))))))

(fn SetWorkingCapacity
  (params (AgeGroup :type AgeGroupEnum%20Enum :default "NewEnumerator0"))
  (if (Utilities|Array|ContainsItem (Variables|Default|GetAgeGroupVeto) AgeGroup)
    (return false)
    (else
      (return true))))

(fn NewPersonInitialize
  (params (Age :type Integer) (Gender :type PopulusGenderEnum%20Enum :default "NewEnumerator0") (MonthOfBirth :type MonthEnum%20Enum :default "NewEnumerator0") (City :type City%20Base%20BP%20Object%20Reference))
  (bind _currentgroup (CallFunction|AgeGroupProcessing Age))
  (bind _returnvalue (Game|SpawnActorfromClass "/Game/Assets/PopulusBP.PopulusBP_C" (Transformation|GetActorTransform City) "Undefined" 0 Age Gender _currentgroup MonthOfBirth (CallFunction|SetWorkingCapacity _currentgroup) self 0))
  (Default|AddingCitizen City _returnvalue)
  (return))