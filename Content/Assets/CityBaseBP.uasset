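; City actor for a turn-based grid strategy game that manages its territory, buildings, population and supplies, with its own UI widget.
; It claims surrounding cells by index math on the controller's flat grid array.
; Citizen labor advances city construction from a DataTable-filtered list, while cell buildings add output to city stock.
; Food demand flags starvation against the faction's provision counter, otherwise draws evenly across stocked food types, redistributing shortfalls.
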(event Custom|OpenCityWidget
  (bind _citywidgetref (Variables|References|GetCityWidgetRef))
  (CallFunction|BuildingListRebuild)
  (Widget|SetVisibility (Variables|References|GetCityWidgetRef) "Visible")
  (Variables|CityStatus|SetIsWidgetOpen true)
  (Variables|/Game/UI-UX/Widgets/CityWidget.CityWidget_C|SetCityRef _citywidgetref self)
  (Default|WidgetCalled _citywidgetref))

(event Custom|CloseCityWidget
  (Widget|SetVisibility (Variables|References|GetCityWidgetRef) "Hidden")
  (Variables|CityStatus|SetIsWidgetOpen false)
  (Default|WidgetDismissed (Variables|References|GetCityWidgetRef)))

(event Custom|CitizensFeeding
  (CallFunction|CityFoodDemand))

(event EventBeginPlay
  (bind _returnvalue (UserInterface|CreateWidget "/Game/UI-UX/Widgets/CityWidget.CityWidget_C" (Game|GetPlayerController 0) self))
  (bind _output_get (Variables|References|SetCityWidgetRef _returnvalue))
  (UserInterface|Viewport|AddtoViewport _output_get 0)
  (Variables|CityStatus|SetIsWidgetOpen false))

(fn ConstructionScript)

(fn VerifyCityZone
  (bind _asturn_based_controller (Utilities|Casting|CastToTurnBasedController (Game|GetPlayerController 0)))
  (while (> (LocalVariables|GetLocalRowCounter) 0)
    (for _index (range (Math|Float|Truncate (|((City-(Y*R))-4) (Math|Conversions|ToFloat(Integer) (Utilities|Array|FindItem (Variables|/Game/CoreBP/TurnBasedController.TurnBasedController_C|GetGridMapArr _asturn_based_controller) (Variables|References|GetCityCellRef))) (Math|Conversions|ToFloat(Integer) (Variables|/Game/CoreBP/TurnBasedController.TurnBasedController_C|GetDimensionY _asturn_based_controller)) (Math|Conversions|ToFloat(Integer) (LocalVariables|GetLocalRowCounter)))) (Math|Float|Truncate (+ (|((City-(Y*R))-4) (Math|Conversions|ToFloat(Integer) (Utilities|Array|FindItem (Variables|/Game/CoreBP/TurnBasedController.TurnBasedController_C|GetGridMapArr _asturn_based_controller) (Variables|References|GetCityCellRef))) (Math|Conversions|ToFloat(Integer) (Variables|/Game/CoreBP/TurnBasedController.TurnBasedController_C|GetDimensionY _asturn_based_controller)) (Math|Conversions|ToFloat(Integer) (LocalVariables|GetLocalRowCounter))) 8.0)))
      (Utilities|Array|AddUnique (Variables|Default|GetCityZoneArr) (Utilities|Array|Get(acopy) (Variables|/Game/CoreBP/TurnBasedController.TurnBasedController_C|GetGridMapArr _asturn_based_controller) _index)))
    (Math|Integer|DecrementInt (LocalVariables|GetLocalRowCounter)))
  (for _index_2 (range (- (Utilities|Array|FindItem (Variables|/Game/CoreBP/TurnBasedController.TurnBasedController_C|GetGridMapArr _asturn_based_controller) (Variables|References|GetCityCellRef)) 4) (Utilities|Array|FindItem (Variables|/Game/CoreBP/TurnBasedController.TurnBasedController_C|GetGridMapArr _asturn_based_controller) (Variables|References|GetCityCellRef)))
    (Utilities|Array|AddUnique (Variables|Default|GetCityZoneArr) (Utilities|Array|Get(acopy) (Variables|/Game/CoreBP/TurnBasedController.TurnBasedController_C|GetGridMapArr _asturn_based_controller) _index_2)))
  (for _index_3 (range (Utilities|Array|FindItem (Variables|/Game/CoreBP/TurnBasedController.TurnBasedController_C|GetGridMapArr _asturn_based_controller) (Variables|References|GetCityCellRef)) (+ (Utilities|Array|FindItem (Variables|/Game/CoreBP/TurnBasedController.TurnBasedController_C|GetGridMapArr _asturn_based_controller) (Variables|References|GetCityCellRef)) 4))
    (Utilities|Array|AddUnique (Variables|Default|GetCityZoneArr) (Utilities|Array|Get(acopy) (Variables|/Game/CoreBP/TurnBasedController.TurnBasedController_C|GetGridMapArr _asturn_based_controller) _index_3)))
  (LocalVariables|SetLocalRowCounter 1)
  (while (< (LocalVariables|GetLocalRowCounter) 5)
    (for _index_4 (range (Math|Float|Truncate (|((City+(Y*R))-4) (Math|Conversions|ToFloat(Integer) (Utilities|Array|FindItem (Variables|/Game/CoreBP/TurnBasedController.TurnBasedController_C|GetGridMapArr _asturn_based_controller) (Variables|References|GetCityCellRef))) (Math|Conversions|ToFloat(Integer) (Variables|/Game/CoreBP/TurnBasedController.TurnBasedController_C|GetDimensionY _asturn_based_controller)) (Math|Conversions|ToFloat(Integer) (LocalVariables|GetLocalRowCounter)))) (Math|Float|Truncate (+ (|((City+(Y*R))-4) (Math|Conversions|ToFloat(Integer) (Utilities|Array|FindItem (Variables|/Game/CoreBP/TurnBasedController.TurnBasedController_C|GetGridMapArr _asturn_based_controller) (Variables|References|GetCityCellRef))) (Math|Conversions|ToFloat(Integer) (Variables|/Game/CoreBP/TurnBasedController.TurnBasedController_C|GetDimensionY _asturn_based_controller)) (Math|Conversions|ToFloat(Integer) (LocalVariables|GetLocalRowCounter))) 8.0)))
      (Utilities|Array|AddUnique (Variables|Default|GetCityZoneArr) (Utilities|Array|Get(acopy) (Variables|/Game/CoreBP/TurnBasedController.TurnBasedController_C|GetGridMapArr _asturn_based_controller) _index_4)))
    (Math|Integer|IncrementInt (LocalVariables|GetLocalRowCounter)))
  (for _array_element (Variables|Default|GetCityZoneArr)
    (Variables|/Game/World/Grid/GridCellBP.GridCellBP_C|SetOwningCity _array_element self))
  (return))

(fn HarvestingSupplies
  (bind _localmonthincome (LocalVariables|GetLocalMonthIncome))
  (bind _localkey (LocalVariables|GetLocalKey))
  (bind _citysuppliesstock (Variables|Default|GetCitySuppliesStock))
  (LocalVariables|SetLocalStock _citysuppliesstock)
  (Utilities|Map|Clear _citysuppliesstock)
  (for _array_element (Variables|Default|GetCellBuildingsArr)
    (if (Variables|/Game/Assets/CellBuildings/CellBuildingBP.CellBuildingBP_C|GetConstructionComplete _array_element)
      (bind _keys (Utilities|Map|Keys (Variables|/Game/Assets/CellBuildings/CellBuildingBP.CellBuildingBP_C|GetResourceOutput _array_element)))
      (for _array_element_2 _keys
        (if (.ReturnValue (Utilities|Map|Find _localmonthincome _array_element_2))
          (bind _output_get (LocalVariables|SetLocalValue (.Value (Utilities|Map|Find _localmonthincome _array_element_2))))
          (Utilities|Map|Remove _localmonthincome _array_element_2)
          (Utilities|Map|Add _localmonthincome _array_element_2 (+ _output_get (.Value (Utilities|Map|Find (Variables|/Game/Assets/CellBuildings/CellBuildingBP.CellBuildingBP_C|GetResourceOutput _array_element) _array_element_2))))
          (else
            (Utilities|Map|Add _localmonthincome _array_element_2 (.Value (Utilities|Map|Find (Variables|/Game/Assets/CellBuildings/CellBuildingBP.CellBuildingBP_C|GetResourceOutput _array_element) _array_element_2))))))
      (else
        (Default|ConstructionProcess _array_element))))
  (bind _keys_2 (Utilities|Map|Keys (LocalVariables|GetLocalStock)))
  (bind _keys_3 (Utilities|Map|Keys (LocalVariables|GetLocalMonthIncome)))
  (for _array_element_3 _keys_2
    (Utilities|Array|AddUnique _localkey _array_element_3))
  (for _array_element_4 _keys_3
    (Utilities|Array|AddUnique _localkey _array_element_4))
  (for _array_element_5 (LocalVariables|GetLocalKey)
    (Utilities|Map|Add (Variables|Default|GetCitySuppliesStock) _array_element_5 (+ (.Value (Utilities|Map|Find (LocalVariables|GetLocalStock) _array_element_5)) (.Value (Utilities|Map|Find (LocalVariables|GetLocalMonthIncome) _array_element_5)))))
  (return (LocalVariables|GetLocalMonthIncome)))

(fn BuildingListInitialize
  (for _array_element (Variables|/Game/Assets/Fractions/FractionBaseBP.FractionBaseBP_C|GetBuildNameList (Variables|References|GetFractionRef))
    (Utilities|Array|Add (Variables|Default|GetCityBuildAvailable) _array_element))
  (CallFunction|BuildingListRebuild)
  (return))

(fn BuildingListRebuild
  (bind _underconstruction (Variables|Default|GetUnderConstruction))
  (if (Utilities|IsValid _underconstruction)
    (if (Utilities|Set|Contains (Variables|/Game/Assets/CityBuildings/CityBuildingBaseBP.CityBuildingBaseBP_C|GetBuildingTags _underconstruction) "NewEnumerator0")
      (for _array_element (Variables|Default|GetCityBuildingsArr) :!label _label
        (bind _array_element_2 (Utilities|Array|ForEachLoopwithBreak (Variables|Default|GetCityBuildAvailable) :!label _label_2)
          (:LoopBody
            (bind _returnvalue (Utilities|GetDataTableRow "/Game/CoreBP/DataBases/CityBuildingsCompositeDT.CityBuildingsCompositeDT" _array_element_2)
              (:then
                (if (Utilities|Enum|Equal(Enum) (.BuildingName (Utilities|Struct|BreakCityBuildingStruct _returnvalue)) (Variables|/Game/Assets/CityBuildings/CityBuildingBaseBP.CityBuildingBaseBP_C|GetBuildingName _array_element))
                  (if (not (Utilities|Set|Contains (Variables|/Game/Assets/CityBuildings/CityBuildingBaseBP.CityBuildingBaseBP_C|GetBuildingTags _array_element) "NewEnumerator0"))
                    (Utilities|Array|RemoveItem (Variables|Default|GetCityBuildAvailable) _array_element_2)
                    (goto _label_2 Break))))))))
      (return)
      (else
        (bind _array_element_3 (Utilities|Array|ForEachLoopwithBreak (Variables|Default|GetCityBuildAvailable) :!label _label_3)
          (:LoopBody
            (bind _returnvalue_2 (Utilities|GetDataTableRow "/Game/CoreBP/DataBases/CityBuildingsCompositeDT.CityBuildingsCompositeDT" _array_element_3)
              (:then
                (if (Utilities|Enum|Equal(Enum) (.BuildingName (Utilities|Struct|BreakCityBuildingStruct _returnvalue_2)) (Variables|/Game/Assets/CityBuildings/CityBuildingBaseBP.CityBuildingBaseBP_C|GetBuildingName _underconstruction))
                  (Utilities|Array|RemoveItem (Variables|Default|GetCityBuildAvailable) _array_element_3)
                  (goto _label_3 Break)))))
          (:Completed
            (goto _label)))))
    (else
      (goto _label))))

(fn AddingCitizen
  (params (Citizen :type Populus%20BP%20Object%20Reference))
  (Utilities|Array|Add (Variables|Default|GetPopulationArr) Citizen)
  (return))

(fn GetLaborPerTurn
  (Variables|Default|SetLaborPerTurn 0.0)
  (for _array_element (Variables|Default|GetPopulationArr)
    (bind _output_get (LocalVariables|SetLocalFloat (Variables|Default|GetLaborPerTurn)))
    (Variables|Default|SetLaborPerTurn (+ _output_get (Variables|/Game/Assets/PopulusBP.PopulusBP_C|GetLabor _array_element))))
  (return))

(fn ConstructionUpdate
  (bind _underconstruction (Variables|Default|GetUnderConstruction))
  (Utilities|IsValid _underconstruction
    (:Is%20Valid
      (bind _output_get (LocalVariables|SetLocalFloat (Variables|/Game/Assets/CityBuildings/CityBuildingBaseBP.CityBuildingBaseBP_C|GetLaborCost _underconstruction)))
      (bind _output_get_2 (Variables|/Game/Assets/CityBuildings/CityBuildingBaseBP.CityBuildingBaseBP_C|SetLaborCost _underconstruction (- _output_get (Variables|Default|GetLaborPerTurn))))
      (if (<= _output_get_2 0.0)
        (CallFunction|ConstructionComplete)
        (return)
        (else
          (Default|ConstructionStatusUpdate (Variables|References|GetCityWidgetRef) _output_get_2)
          (return))))))

(fn ConstructionComplete
  (bind _citywidgetref (Variables|References|GetCityWidgetRef))
  (Utilities|Array|Add (Variables|Default|GetCityBuildingsArr) (Variables|Default|GetUnderConstruction))
  (Widget|Panel|ClearChildren (Variables|/Game/UI-UX/Widgets/CityWidget.CityWidget_C|GetOnConstructBox _citywidgetref))
  (Variables|/Game/UI-UX/Widgets/CityWidget.CityWidget_C|SetConstructedWidget _citywidgetref 0)
  (Variables|Default|SetUnderConstruction 0)
  (return))

(fn HarvestInternalResources
  (bind _localstock (LocalVariables|GetLocalStock))
  (for _array_element (Variables|Default|GetCityBuildingsArr)
    (bind _keys (Utilities|Map|Keys (Variables|/Game/Assets/CityBuildings/CityBuildingBaseBP.CityBuildingBaseBP_C|GetResourceOutput _array_element)))
    (for _array_element_2 _keys
      (if (Utilities|Map|Contains _localstock _array_element_2)
        (bind _output_get (LocalVariables|SetLocalValue (.Value (Utilities|Map|Find _localstock _array_element_2))))
        (Utilities|Map|Remove _localstock _array_element_2)
        (Utilities|Map|Add _localstock _array_element_2 (+ (.Value (Utilities|Map|Find (Variables|/Game/Assets/CityBuildings/CityBuildingBaseBP.CityBuildingBaseBP_C|GetResourceOutput _array_element) _array_element_2)) _output_get))
        (else
          (Utilities|Map|Add _localstock _array_element_2 (.Value (Utilities|Map|Find (Variables|/Game/Assets/CityBuildings/CityBuildingBaseBP.CityBuildingBaseBP_C|GetResourceOutput _array_element) _array_element_2)))))))
  (return (LocalVariables|GetLocalStock)))

(fn CityFoodDemand
  (bind _citysuppliesstock (Variables|Default|GetCitySuppliesStock))
  (bind _localstock (LocalVariables|GetLocalStock))
  (bind _citysuppliesstock_2 (Variables|Default|GetCitySuppliesStock))
  (bind _fractionref (Variables|References|GetFractionRef))
  (bind _citysuppliesstock_3 (Variables|Default|GetCitySuppliesStock))
  (bind _resourcecounter (Variables|/Game/Assets/Fractions/FractionBaseBP.FractionBaseBP_C|GetResourceCounter _fractionref))
  (bind _value (Utilities|Map|Find _resourcecounter "Proviancy"))
  (for _array_element (Variables|Default|GetCellBuildingsArr)
    (for _array_element_2 (Variables|/Game/Assets/CellBuildings/CellBuildingBP.CellBuildingBP_C|GetCellBuildingWorkers _array_element)
      (LocalVariables|SetLocalConsumption (+ (Variables|/Game/Assets/PopulusBP.PopulusBP_C|GetFoodConsumption _array_element_2) (LocalVariables|GetLocalConsumption)))))
  (for _array_element_3 (Variables|Default|GetPopulationArr)
    (LocalVariables|SetLocalConsumption (+ (Variables|/Game/Assets/PopulusBP.PopulusBP_C|GetFoodConsumption _array_element_3) (LocalVariables|GetLocalConsumption))))
  (if (> (LocalVariables|GetLocalConsumption) _value)
    (Variables|Default|SetIsStarving (> (LocalVariables|GetLocalConsumption) _value))
    (Variables|Default|SetStarvingCounter (- (LocalVariables|GetLocalConsumption) _value))
    (for _array_element_4 (Variables|/Game/Assets/Resources/ResourceBaseBP.ResourceBaseBP_C|GetIncludedResources (Variables|/Game/Assets/Fractions/FractionBaseBP.FractionBaseBP_C|GetProviancyRef (Variables|References|GetFractionRef)))
      (LocalVariables|SetLocalConsumption (- (LocalVariables|GetLocalConsumption) (.Value (Utilities|Map|Find _citysuppliesstock _array_element_4))))
      (Utilities|Map|Remove _citysuppliesstock _array_element_4))
    (return)
    (else
      (for _array_element_5 (Variables|/Game/Assets/Resources/ResourceBaseBP.ResourceBaseBP_C|GetIncludedResources (Variables|/Game/Assets/Fractions/FractionBaseBP.FractionBaseBP_C|GetProviancyRef (Variables|References|GetFractionRef)))
        (if (.ReturnValue (Utilities|Map|Find (Variables|Default|GetCitySuppliesStock) _array_element_5))
          (Math|Float|IncrementFloat (LocalVariables|GetLocalSupplyType))))
      (LocalVariables|SetLocalShare (Math|Conversions|ToFloat(Integer) (Math|Float|Floor (/ (LocalVariables|GetLocalConsumption) (LocalVariables|GetLocalSupplyType)))))
      (for _array_element_6 (Variables|/Game/Assets/Resources/ResourceBaseBP.ResourceBaseBP_C|GetIncludedResources (Variables|/Game/Assets/Fractions/FractionBaseBP.FractionBaseBP_C|GetProviancyRef (Variables|References|GetFractionRef)))
        (if (.ReturnValue (Utilities|Map|Find _citysuppliesstock_3 _array_element_6))
          (if (<= (LocalVariables|GetLocalShare) (.Value (Utilities|Map|Find _citysuppliesstock_3 _array_element_6)))
            (Utilities|Map|Add (LocalVariables|GetLocalStock) _array_element_6 (- (.Value (Utilities|Map|Find _citysuppliesstock_3 _array_element_6)) (LocalVariables|GetLocalShare)))
            (Utilities|Map|Remove _citysuppliesstock_3 _array_element_6)
            (else
              (LocalVariables|SetLocalRemain (+ (- (LocalVariables|GetLocalShare) (.Value (Utilities|Map|Find _citysuppliesstock_3 _array_element_6))) (LocalVariables|GetLocalRemain)))
              (Utilities|Map|Remove _citysuppliesstock_3 _array_element_6)))))
      (bind _keys (Utilities|Map|Keys _localstock))
      (for _array_element_7 _keys
        (Utilities|Map|Add (Variables|Default|GetCitySuppliesStock) _array_element_7 (.Value (Utilities|Map|Find _localstock _array_element_7))))
      (if (> (LocalVariables|GetLocalRemain) 0.0)
        (bind _array_element_8 (Utilities|Array|ForEachLoopwithBreak (Variables|/Game/Assets/Resources/ResourceBaseBP.ResourceBaseBP_C|GetIncludedResources (Variables|/Game/Assets/Fractions/FractionBaseBP.FractionBaseBP_C|GetProviancyRef (Variables|References|GetFractionRef))) :!label _label)
          (:LoopBody
            (if (> (LocalVariables|GetLocalRemain) 0.0)
              (if (.ReturnValue (Utilities|Map|Find _citysuppliesstock_2 _array_element_8))
                (if (>= (LocalVariables|GetLocalRemain) (.Value (Utilities|Map|Find _citysuppliesstock_2 _array_element_8)))
                  (LocalVariables|SetLocalRemain (- (LocalVariables|GetLocalRemain) (.Value (Utilities|Map|Find _citysuppliesstock_2 _array_element_8))))
                  (else
                    (Utilities|Map|Add (LocalVariables|GetLocalStock) _array_element_8 (- (.Value (Utilities|Map|Find _citysuppliesstock_2 _array_element_8)) (LocalVariables|GetLocalRemain)))
                    (Utilities|Map|Remove _citysuppliesstock_2 _array_element_8)
                    (LocalVariables|SetLocalRemain 0.0)
                    (goto _label Break))))
              (else
                (goto _label Break))))
          (:Completed
            (return)))))))